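; Pistol weapon Blueprint for the battle royale mode, extending a parent weapon class.
; Fire and Reload defer to the parent, with firing also increasing hip-fire spread.
; Overrides weapon change by ID to store the pistol ID and set the skeletal mesh, with a switch on the pistol ID enum set up for more variants but currently using the 1911 mesh.
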(event `self.ReceiveBeginPlay`
  (`parent.ReceiveBeginPlay`))

(event `self.Fire`
  (`parent.Fire`)
  (`self.IncreaseSpread` 0.1))

(event `self.Reload`
  (`parent.Reload`))

(event `self.ChangeWeaponOnID`
  (params (WeaponID :type Integer))
  ;[1 1 1] Change Weapon On ID Override
  (bind _output_get (set `self.WeaponID` WeaponID))
  ;;[0.1019 1 0.2207] Add more pins based on ENUM_PistolWeaponID to change weapon
  (switch `int` _output_get
    (:`1`
      ;;;[1 1 1] Base Mesh
      (`SkinnedMeshComponent.SetSkinnedAssetAndUpdate` (`self.WeaponMesh`) "/Game/BattleRoyale/Meshes/Pistol/SKM_1911.SKM_1911" true))))

(fn `UserConstructionScript`
  (`parent.UserConstructionScript`))